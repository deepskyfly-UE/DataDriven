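; BP_Dropper is a test actor for data assets that spawns a drop item whenever it is hit.
; On Hit it async loads the soft-referenced ItemType, casts it to ShopItemAsset, and passes it to a new BP_DropItem spawned at SpawnOrigin.
; The construction script shows the ItemType reference on a text render component, labeling what each dropper produces.
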(event `self.ReceiveHit`
  (params (MyComp :type "PrimitiveComponent Object Reference") (Other :type "Actor Object Reference") (OtherComp :type "PrimitiveComponent Object Reference") (bSelfMoved :type Boolean) (HitLocation :type "Vector Structure") (HitNormal :type "Vector Structure") (NormalImpulse :type "Vector Structure") (Hit :type "HitResult Structure (by ref)"))
  (bind _object (`|LoadAsset` (`KismetSystemLibrary.Conv_SoftObjPathToSoftObjRef` (`self.ItemType`)))
    (:`Completed`
      (bind _asshop_item_asset (cast `ShopItemAsset` _object))
      (`|SpawnActorFromClass` "/Game/Blueprint/Test/DataAssetTest/BP_DropItem.BP_DropItem_C" (`SceneComponent.K2_GetComponentToWorld` (`self.SpawnOrigin`)) "Undefined" "OverrideRootScale" null _asshop_item_asset null))))

(fn `UserConstructionScript`
  (`TextRenderComponent.K2_SetText` (`self.TextRender`) (`KismetTextLibrary.Conv_StringToText` (`KismetSystemLibrary.Conv_SoftObjectReferenceToString` (`KismetSystemLibrary.Conv_SoftObjPathToSoftObjRef` (`self.ItemType`))))))