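; Test actor that drives the vertical scale of its Cone component from an Excel spreadsheet.
; On BeginPlay it loads ShopItems.xlsx from a hardcoded absolute path and applies cell C3 of the active sheet as the cone's Z scale.
; It then watches the workbook with auto-reload, and a change callback reapplies that cell so spreadsheet edits show up during play.
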(event `self.ReceiveBeginPlay`
  (bind _returnvalue (`DirectExcelLibrary.LoadExcel` "E:\\Workspace\\DataDriven\\Data\\ShopItems.xlsx"))
  (`|ExecutionSequence`
    (:`then_0`
      (`SceneComponent.SetRelativeScale3D` (`self.Cone`) (`KismetMathLibrary.MakeVector` 1.0 1.0 (`ExcelCell.ToFloat` (`ExcelWorksheet.CellAtId` (`ExcelWorkbook.ActiveSheet` _returnvalue) "C3")))))
    (:`then_1`
      (`ExcelWorkbook.StartWatch` _returnvalue (delegate `CustomEvent_0`) true 1.0))))

(event `CustomEvent_0`
  (params (workbook :type "ExcelWorkbook Object Reference"))
  (`SceneComponent.SetRelativeScale3D` (`self.Cone`) (`KismetMathLibrary.MakeVector` 1.0 1.0 (`ExcelCell.ToFloat` (`ExcelWorksheet.CellAtId` (`ExcelWorkbook.ActiveSheet` workbook) "C3")))))

(fn `UserConstructionScript`)